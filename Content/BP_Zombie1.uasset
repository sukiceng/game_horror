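; Zombie AI pawn that roams at random and moves toward pawns it spots.
; A self-restarting AI MoveTo loop picks reachable points around its current location, pausing briefly after each success and retrying immediately on failure.
; Pawn Sensing triggers a separate MoveTo toward the seen pawn.
; No state gates the two behaviors, so an interrupted wander move restarts wandering and can override the chase.
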(event OnSeePawn(PawnSensing)
  (params (Pawn :type Pawn%20Object%20Reference))
  (CallFunction|ChaseTarget Pawn))

(event Custom|Zombie1
  (AI|AIMoveTo self (.RandomLocation (AI|Navigation|GetRandomReachablePointinRadius (Transformation|GetActorLocation) 2e+03 0 0)) 0 5.0 false
    (:OnSuccess
      (Utilities|FlowControl|Delay 0.8))
    (:OnFail
      _))
  (CallFunction|Zombie1))

(event Custom|Chase%20Target
  (params (TargetActor :type Actor%20Object%20Reference))
  (AI|AIMoveTo self "0, 0, 0" TargetActor 1.2e+02 false))

(event EventBeginPlay
  (CallFunction|Zombie1))

(fn ConstructionScript)